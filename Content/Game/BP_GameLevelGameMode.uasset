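; Game mode for the game level that numbers joining players and splits their spawns between two Player Starts.
; HandleStartingNewPlayer calls the parent, increments PlayerNum, prints the count and stores it in the player's BP_PlayerState.
; ChoosePlayerStart uses PlayerNum parity to return the first (even) or second (odd) PlayerStart found by GetAllActorsOfClass, so placement depends on that array's order.
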(event EventHandleStartingNewPlayer
  (params (NewPlayer :type Player%20Controller%20Object%20Reference))
  (|CallParentFunction NewPlayer)
  (bind _result (Math|Integer|IncrementInt (Variables|Default|GetPlayerNum))
    (:%20%20
      (Development|PrintString (Utilities|String|Append (Utilities|String|ToString(Integer) _result) "명"))
      (bind _asbp_player_state (Utilities|Casting|CastToBP_PlayerState (Variables|/Script/Engine.Controller|GetPlayerState NewPlayer)))
      (Variables|/Game/Game/BP_PlayerState.BP_PlayerState_C|SetPlayerNum _asbp_player_state _result))))

(fn ConstructionScript)

(fn ChoosePlayerStart
  (params (Player :type Controller%20Object%20Reference))
  (if (== (Math|Integer|%(Integer) (Variables|Default|GetPlayerNum) 2) 0)
    (bind _outactors (Actor|GetAllActorsOfClass "/Script/Engine.PlayerStart"))
    (for (_array_element _array_index) _outactors
      (if (== _array_index 0)
        (return _array_element)))
    (else
      (bind _outactors_2 (Actor|GetAllActorsOfClass "/Script/Engine.PlayerStart"))
      (for (_array_element_2 _array_index_2) _outactors_2
        (if (== _array_index_2 1)
          (return _array_element_2))))))