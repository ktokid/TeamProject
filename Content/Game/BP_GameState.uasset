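; Game State Blueprint that flags the game as started when play begins.
; BeginPlay caches the level HUD and its timer and countdown widgets, then, on authority only, resets the started and countdown flags in BP_TeamProjectInstance.
; Per-interval elapsed-time and final-minute countdown functions remain but are never run; a note says sync problems were solved in the game instance instead.
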(event EventBeginPlay
  (Utilities|FlowControl|Sequence
    (:then_0
      ;[1 1 1] GameHud Widget 변수 만듦
      (CallFunction|Initialize)
      ;[1 1 1] 주의 여기에 Authority switch 있다
      (CallFunction|SetGameStartedatGameInstance))))

(fn ConstructionScript)

(fn EverySeconds
  ;[1 1 1] 로직과 싱크 문제가 있는데 어떻게 해결해야 할지 몰라서 게임인스턴스에서 해결했다 . 실행 되지 않는다
  (Variables|Default|SetDeltaSeconds (+ (Variables|Default|GetIntervalSeconds) (Variables|Default|GetDeltaSeconds)))
  (if (Ability|HasAuthority)
    _
    (else
      _))
  (if (and (<= (- (Math|Conversions|ToFloat(Integer) (Variables|Default|GetCountDownFrom)) (Variables|Default|GetDeltaSeconds)) 6e+01) (> (- (Math|Conversions|ToFloat(Integer) (Variables|Default|GetCountDownFrom)) (Variables|Default|GetDeltaSeconds)) 0.0))
    (Variables|Default|SetCountDownStart true)
    (else
      (Variables|Default|SetCountDownStart false)))
  (Default|ShowTimer (Variables|Default|GetBP_GameLevelHud))
  (Default|ShowCountDown (Variables|Default|GetBP_GameLevelHud)))

(fn Initialize
  (bind _asbp_game_level_hud (Utilities|Casting|CastToBP_GameLevelHud (HUD|GetHUD (Game|GetPlayerController 0))))
  (bind _output_get (Variables|Default|SetBP_GameLevelHud _asbp_game_level_hud))
  (bind _output_get_2 (Variables|Default|SetWGGameLevel (Variables|/Game/Taeryong/Game/BP_GameLevelHud.BP_GameLevelHud_C|GetWG_GameLevel _output_get)))
  (Variables|Default|SetCountDownWidget (Variables|/Game/Taeryong/Game/Widget/WG_GameLevel.WG_GameLevel_C|GetCountDownWidget _output_get_2))
  (Variables|Default|SetTimerWidget (Variables|/Game/Taeryong/Game/Widget/WG_GameLevel.WG_GameLevel_C|GetTimerWidget (Variables|/Game/Taeryong/Game/BP_GameLevelHud.BP_GameLevelHud_C|GetWG_GameLevel _output_get)))
  (Variables|Default|SetTimeLapseWidgetGame (Variables|/Game/Taeryong/Game/Widget/WG_GameLevel.WG_GameLevel_C|GetTimeLapseWidget_Game (Variables|/Game/Taeryong/Game/BP_GameLevelHud.BP_GameLevelHud_C|GetWG_GameLevel _output_get))))

(fn ShowTimer
  (bind _deltaseconds (Variables|Default|GetDeltaSeconds))
  (bind _timerwidget (Variables|Default|GetTimerWidget))
  (bind _outputtext (CallFunction|TimetoWidget (Math|Float|%(Float) _deltaseconds 6e+01)))
  (Variables|/Game/Taeryong/Game/Widget/TimerWidget.TimerWidget_C|SetStrElapsedSecondes _timerwidget _outputtext)
  (bind _outputtext_2 (CallFunction|TimetoWidget (Math|Float|%(Float) (Math|Conversions|ToFloat(Integer) (.ReturnValue (Math|Float|Division(WholeandRemainder) _deltaseconds 6e+01))) 6e+01)))
  (Variables|/Game/Taeryong/Game/Widget/TimerWidget.TimerWidget_C|SetStrElapsedMinutes _timerwidget _outputtext_2)
  (bind _outputtext_3 (CallFunction|TimetoWidget (Math|Float|%(Float) (Math|Conversions|ToFloat(Integer) (.ReturnValue (Math|Float|Division(WholeandRemainder) _deltaseconds 3.6e+03))) 24.0)))
  (Variables|/Game/Taeryong/Game/Widget/TimerWidget.TimerWidget_C|SetStrElapsedHours _timerwidget _outputtext_3)
  (bind _outputtext_4 (CallFunction|InttoText (.ReturnValue (Math|Float|Division(WholeandRemainder) _deltaseconds 8.64e+04))))
  (Variables|/Game/Taeryong/Game/Widget/TimerWidget.TimerWidget_C|SetStrElapsedDays _timerwidget _outputtext_4))

(fn TimetoWidget
  (params (InputFloat :type Float%20%28single-precision%29))
  (bind _outintger (CallFunction|FloattoInt InputFloat))
  (bind _outputtext (CallFunction|InttoText _outintger))
  (return _outputtext))

(fn FloattoInt
  (params (InputFloat :type Float%20%28single-precision%29))
  (return (Math|Float|Truncate InputFloat)))

(fn InttoText
  (params (InputInteger :type Integer))
  (return (Utilities|Text|ToText(Integer) InputInteger)))

(fn NewFunction0)

(fn ShowCountDown
  (bind _countdownfrom (Variables|Default|GetCountDownFrom))
  (bind _deltaseconds (Variables|Default|GetDeltaSeconds))
  (bind _returnvalue (Math|Conversions|ToFloat(Integer) _countdownfrom))
  (bind _returnvalue_2 (- _returnvalue _deltaseconds))
  (if (and (<= _returnvalue_2 6e+01) (> _returnvalue_2 0.0))
    (Default|ShowCountDown (Variables|Default|GetCountDownWidget) (Utilities|Text|ToText(Float) _returnvalue_2 "HalfToEven"))
    (elif (<= _returnvalue_2 0.0)
      _)))

(fn SetGameStartedatGameInstance
  (if (Ability|HasAuthority)
    (bind _asbp_team_project_instance (Utilities|Casting|CastToBP_TeamProjectInstance (Game|GetGameInstance)))
    (Variables|/Game/Taeryong/BP_TeamProjectInstance.BP_TeamProjectInstance_C|SetIsGameStarted _asbp_team_project_instance true)
    (Variables|/Game/Taeryong/BP_TeamProjectInstance.BP_TeamProjectInstance_C|SetIsCountDownEnd _asbp_team_project_instance false)
    (Variables|/Game/Taeryong/BP_TeamProjectInstance.BP_TeamProjectInstance_C|SetIsCountDownStart _asbp_team_project_instance false)))