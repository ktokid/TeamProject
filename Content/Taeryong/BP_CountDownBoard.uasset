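; BP_CountDownBoard is a board that displays a countdown through a TextRender, refreshed every Tick.
; On authority, BeginPlay seeds CountDown from BP_GameState and starts a looping one-second UpdateTimer.
; UpdateTimer decrements toward zero only while BP_TeamProjectInstance flags the countdown as started and not ended.
; ClearUpdateTimer stops the timer on request; reaching zero does not clear it.
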(event Custom|UpdateTimer
  (bind _asbp_team_project_instance (Utilities|Casting|CastToBP_TeamProjectInstance (Game|GetGameInstance)))
  (if (and (Variables|/Game/Taeryong/BP_TeamProjectInstance.BP_TeamProjectInstance_C|GetIsCountDownStart _asbp_team_project_instance) (not (Variables|/Game/Taeryong/BP_TeamProjectInstance.BP_TeamProjectInstance_C|GetIsCountDownEnd _asbp_team_project_instance)))
    (if (> (Variables|Default|GetCountDown) 0)
      (Variables|Default|SetCountDown (- (Variables|Default|GetCountDown) 1))
      (bind _asbp_team_project_instance_2 (Utilities|Casting|CastToBP_TeamProjectInstance (Game|GetGameInstance)))
      (if (Variables|/Game/Taeryong/BP_TeamProjectInstance.BP_TeamProjectInstance_C|GetIsCountDownEnd _asbp_team_project_instance_2)
        (Utilities|Time|ClearTimerbyFunctionName 0 "UpdateTimer")))))

(event EventBeginPlay
  (Networking|SwitchHasAuthority
    (:Authority
      (bind _asbp_game_state (Utilities|Casting|CastToBP_GameState (Game|GetGameState)))
      (Variables|Default|SetCountDown (Variables|/Game/Game/BP_GameState.BP_GameState_C|GetCountDownFrom _asbp_game_state))
      (Utilities|Time|SetTimerbyFunctionName 0 "UpdateTimer" 1.0 true))))

(event EventTick
  (params (DeltaSeconds :type Float%20%28single-precision%29))
  (Rendering|Components|TextRender|SetText (Variables|Default|GetTextRender) (Utilities|Text|ToText(Integer) (Variables|Default|GetCountDown))))

(fn ConstructionScript)

(fn ClearUpdateTimer
  (Utilities|Time|ClearTimerbyFunctionName 0 "UpdateTimer"))