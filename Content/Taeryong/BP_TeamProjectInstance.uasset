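; Game instance that tracks time elapsed since launch and drives the match countdown.
; A looping one-second timer advances DeltaSeconds, an accumulated clock scaled by a multiplier, and records its value when the game starts.
; Each tick detects the Entry, Lobby or Game HUD and writes days/hours/minutes/seconds to its time-lapse widget.
; It also compares time since game start with GameState's CountDownFrom, calling countdown start each tick within the final minute and end once below zero.
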(event EventInit
  ;[1 1 1] 게임 접속 부터 경과 시간 보여 줌
  (CallFunction|EverySeconds)
  (Utilities|Time|SetTimerbyFunctionName 0 "EverySeconds" 1.0 true))

(fn EverySeconds
  (Utilities|FlowControl|Sequence
    (:then_0
      (if (and (Variables|Default|GetIsGameStarted) (not (Variables|Default|GetGameStartDeltaSecondsStored)))
        (Variables|Default|SetGameStartDeltaSeconds (Variables|Default|GetDeltaSeconds))
        (Variables|Default|SetGameStartDeltaSecondsStored true))
      (Variables|Default|SetDeltaSeconds (+ (* 1.0 (Variables|Default|GetDeltaSecondsMultiples)) (Variables|Default|GetDeltaSeconds)))
      ;[1 1 1] 게임 시간을 뿌려줄 허드와 위젯을 결정하고 변수로 만든다
      (CallFunction|CheckWheretoCast)
      (switch Utilities|FlowControl|Switch|SwitchonEN_ModeSelection (Variables|Default|GetEN_GameModeSelection)
        (:NewEnumerator0
          (CallFunction|ShowDDHHMMSS))
        (:NewEnumerator1
          (CallFunction|ShowDDHHMMSSLobby))
        (:NewEnumerator2
          (CallFunction|ShowDDHHMMSSGameLevel))))
    (:then_1
      (if (not (Variables|Default|GetIsCountDownEnd))
        (bind _asbp_game_state (Utilities|Casting|CastToBP_GameState (Game|GetGameState)))
        (if (Math|Boolean|ANDBoolean (and (>= (- (Variables|/Game/Game/BP_GameState.BP_GameState_C|GetCountDownFrom _asbp_game_state) (Math|Float|Truncate (- (Variables|Default|GetDeltaSeconds) (Variables|Default|GetGameStartDeltaSeconds)))) 0) (<= (- (Variables|/Game/Game/BP_GameState.BP_GameState_C|GetCountDownFrom _asbp_game_state) (Math|Float|Truncate (- (Variables|Default|GetDeltaSeconds) (Variables|Default|GetGameStartDeltaSeconds)))) 60)) (Variables|Default|GetIsGameStarted) (Variables|Default|GetGameStartDeltaSecondsStored))
          (Variables|Default|SetIsCountDownStart true)
          (Default|CallEventDispatcherCountDownStart (Variables|/Game/Game/BP_GameState.BP_GameState_C|GetCountDownFrom _asbp_game_state))
          (elif (< (- (Variables|/Game/Game/BP_GameState.BP_GameState_C|GetCountDownFrom _asbp_game_state) (Math|Float|Truncate (- (Variables|Default|GetDeltaSeconds) (Variables|Default|GetGameStartDeltaSeconds)))) 0)
            (Variables|Default|SetIsCountDownEnd true)
            (Default|CallEventDispacherCountDownEnd)
            (Development|PrintString "CountEnd" true true "(R=0.167905,G=0.227356,B=1.000000,A=1.000000)" 1e+01)
            (else
              (Variables|Default|SetIsCountDownEnd false))))))))

(fn FloortoInt
  (params (InputFloat :type Float%20%28single-precision%29))
  (return (Math|Float|Truncate InputFloat)))

(fn InttoText
  (params (InputInteger :type Integer))
  (return (Utilities|Text|ToText(Integer) InputInteger)))

(fn TimetoWidget
  (params (InputFloat :type Float%20%28single-precision%29))
  (bind _outputinteger (CallFunction|FloortoInt InputFloat))
  (bind _outtext (CallFunction|InttoText _outputinteger))
  (return _outtext))

(fn CheckWheretoCast
  (bind _asbp_entry_hud (Utilities|Casting|CastToBP_EntryHud (HUD|GetHUD (Game|GetPlayerController 0)))
    (:then
      (Utilities|IsValid _asbp_entry_hud
        (:Is%20Valid
          (Variables|Default|SetEN_GameModeSelection "NewEnumerator0")
          (bind _output_get (Variables|Default|SetEntry_Widget (Variables|/Game/Taeryong/Entry/BP_EntryHud.BP_EntryHud_C|GetWG_Entry _asbp_entry_hud)))
          (Variables|Default|SetTimeLapseWidget (Variables|/Game/Taeryong/Entry/Widget/WG_Entry.WG_Entry_C|GetTimeLapseWidget _output_get)))
        (:Is%20Not%20Valid
          (bind _asbp_game_level_hud (Utilities|Casting|CastToBP_GameLevelHud (HUD|GetHUD (Game|GetPlayerController 0)) :!label _label)
            (:then
              (Utilities|IsValid _asbp_game_level_hud
                (:Is%20Valid
                  (Variables|Default|SetEN_GameModeSelection "NewEnumerator2")
                  (bind _output_get_2 (Variables|Default|SetWG_GameLevel (Variables|/Game/Taeryong/Game/BP_GameLevelHud.BP_GameLevelHud_C|GetWG_GameLevel _asbp_game_level_hud)))
                  (Variables|Default|SetTimeLapseWidget_GameLevel (Variables|/Game/Taeryong/Game/Widget/WG_GameLevel.WG_GameLevel_C|GetTimeLapseWidget_Game _output_get_2)))))
            (:CastFailed
              (bind _asbp_lobby_hud (Utilities|Casting|CastToBP_LobbyHud (HUD|GetHUD (Game|GetPlayerController 0))))
              (Utilities|IsValid _asbp_lobby_hud
                (:Is%20Valid
                  (Variables|Default|SetEN_GameModeSelection "NewEnumerator1")
                  (bind _output_get_3 (Variables|Default|SetWG_Lobby (Variables|/Game/Taeryong/Lobby/BP_LobbyHud.BP_LobbyHud_C|GetWG_Lobby _asbp_lobby_hud)))
                  (Variables|Default|SetTimeLapseWidget_Lobby (Variables|/Game/Taeryong/Lobby/WG_Lobby.WG_Lobby_C|GetTimeLapseWidget_Lobby _output_get_3)))
                (:Is%20Not%20Valid
                  (Variables|Default|SetEN_GameModeSelection "NewEnumerator3"))))))))
    (:CastFailed
      (goto _label))))

(fn ShowDDHHMMSS
  (bind _timelapsewidget (Variables|Default|GetTimeLapseWidget))
  (bind _outtext (CallFunction|TimetoWidget (Math|Float|%(Float) (Variables|Default|GetDeltaSeconds) 6e+01)))
  (Variables|/Game/Taeryong/Entry/Widget/TimeLapseWidget.TimeLapseWidget_C|SetStrElapsedSecondes _timelapsewidget _outtext)
  (bind _outtext_2 (CallFunction|TimetoWidget (Math|Float|%(Float) (Math|Conversions|ToFloat(Integer) (.ReturnValue (Math|Float|Division(WholeandRemainder) (Variables|Default|GetDeltaSeconds) 6e+01))) 6e+01)))
  (Variables|/Game/Taeryong/Entry/Widget/TimeLapseWidget.TimeLapseWidget_C|SetStrElapsedMinutes _timelapsewidget _outtext_2)
  (bind _outtext_3 (CallFunction|TimetoWidget (Math|Float|%(Float) (Math|Conversions|ToFloat(Integer) (.ReturnValue (Math|Float|Division(WholeandRemainder) (Variables|Default|GetDeltaSeconds) 3.6e+03))) 24.0)))
  (Variables|/Game/Taeryong/Entry/Widget/TimeLapseWidget.TimeLapseWidget_C|SetStrElapsedHours _timelapsewidget _outtext_3)
  (bind _outtext_4 (CallFunction|InttoText (.ReturnValue (Math|Float|Division(WholeandRemainder) (Variables|Default|GetDeltaSeconds) 8.64e+04))))
  (Variables|/Game/Taeryong/Entry/Widget/TimeLapseWidget.TimeLapseWidget_C|SetStrElapsedDays _timelapsewidget _outtext_4))

(fn ShowDDHHMMSSGameLevel
  (bind _timelapsewidget_gamelevel (Variables|Default|GetTimeLapseWidget_GameLevel))
  (bind _outtext (CallFunction|TimetoWidget (Math|Float|%(Float) (Variables|Default|GetDeltaSeconds) 6e+01)))
  (Variables|/Game/Taeryong/Entry/Widget/TimeLapseWidget.TimeLapseWidget_C|SetStrElapsedSecondes _timelapsewidget_gamelevel _outtext)
  (bind _outtext_2 (CallFunction|TimetoWidget (Math|Float|%(Float) (Math|Conversions|ToFloat(Integer) (.ReturnValue (Math|Float|Division(WholeandRemainder) (Variables|Default|GetDeltaSeconds) 6e+01))) 6e+01)))
  (Variables|/Game/Taeryong/Entry/Widget/TimeLapseWidget.TimeLapseWidget_C|SetStrElapsedMinutes _timelapsewidget_gamelevel _outtext_2)
  (bind _outtext_3 (CallFunction|TimetoWidget (Math|Float|%(Float) (Math|Conversions|ToFloat(Integer) (.ReturnValue (Math|Float|Division(WholeandRemainder) (Variables|Default|GetDeltaSeconds) 3.6e+03))) 24.0)))
  (Variables|/Game/Taeryong/Entry/Widget/TimeLapseWidget.TimeLapseWidget_C|SetStrElapsedHours _timelapsewidget_gamelevel _outtext_3)
  (bind _outtext_4 (CallFunction|InttoText (.ReturnValue (Math|Float|Division(WholeandRemainder) (Variables|Default|GetDeltaSeconds) 8.64e+04))))
  (Variables|/Game/Taeryong/Entry/Widget/TimeLapseWidget.TimeLapseWidget_C|SetStrElapsedDays _timelapsewidget_gamelevel _outtext_4))

(fn ShowDDHHMMSSLobby
  (bind _timelapsewidget_lobby (Variables|Default|GetTimeLapseWidget_Lobby))
  (bind _outtext (CallFunction|TimetoWidget (Math|Float|%(Float) (Variables|Default|GetDeltaSeconds) 6e+01)))
  (Variables|/Game/Taeryong/Lobby/TimeLapseWidget_Lobby.TimeLapseWidget_Lobby_C|SetStrElapsedSecondes _timelapsewidget_lobby _outtext)
  (bind _outtext_2 (CallFunction|TimetoWidget (Math|Float|%(Float) (Math|Conversions|ToFloat(Integer) (.ReturnValue (Math|Float|Division(WholeandRemainder) (Variables|Default|GetDeltaSeconds) 6e+01))) 6e+01)))
  (Variables|/Game/Taeryong/Lobby/TimeLapseWidget_Lobby.TimeLapseWidget_Lobby_C|SetStrElapsedMinutes _timelapsewidget_lobby _outtext_2)
  (bind _outtext_3 (CallFunction|TimetoWidget (Math|Float|%(Float) (Math|Conversions|ToFloat(Integer) (.ReturnValue (Math|Float|Division(WholeandRemainder) (Variables|Default|GetDeltaSeconds) 3.6e+03))) 24.0)))
  (Variables|/Game/Taeryong/Lobby/TimeLapseWidget_Lobby.TimeLapseWidget_Lobby_C|SetStrElapsedHours _timelapsewidget_lobby _outtext_3)
  (bind _outtext_4 (CallFunction|InttoText (.ReturnValue (Math|Float|Division(WholeandRemainder) (Variables|Default|GetDeltaSeconds) 8.64e+04))))
  (Variables|/Game/Taeryong/Lobby/TimeLapseWidget_Lobby.TimeLapseWidget_Lobby_C|SetStrElapsedDays _timelapsewidget_lobby _outtext_4))