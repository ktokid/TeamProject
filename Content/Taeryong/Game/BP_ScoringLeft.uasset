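; BP_ScoringLeft is a left-side scoring trigger that shows its count on a RotatingScore widget.
; On the server, an overlap of its Cube by player 0's BP_Character increments ScoreLeft.
; The RepNotify on ScoreLeft updates the widget text and fires the UpdateCountLeft dispatcher.
; A looping timer turns the widget toward the local camera and refreshes the displayed score.
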(event OnComponentBeginOverlap(Cube)
  (params (OverlappedComponent :type Primitive%20Component%20Object%20Reference) (OtherActor :type Actor%20Object%20Reference) (OtherComp :type Primitive%20Component%20Object%20Reference) (OtherBodyIndex :type Integer) (bFromSweep :type Boolean) (SweepResult :type Hit%20Result%20Structure%20%28by%20ref%29))
  ;[1 1 1] 서버에서만 실행하는지 체크
  (Networking|SwitchHasAuthority
    (:Authority
      ;[1 1 1] 게임에 맞게 바꿔야 한다.
      (bind _asbp_character (Utilities|Casting|CastToBP_Character (Game|Player|GetPlayerPawn 0)))
      (if (== _asbp_character OtherActor)
        ;[1 0 0] ServerCountingUpdate
        (CallFunction|UpdatingCountingLeft)
        (Development|PrintString (Utilities|String|ToString(Integer) (Variables|Default|GetScoreLeft)))))))

(event EventBeginPlay
  (bind _asrotating_score (Utilities|Casting|CastToRotatingScore (UserInterface|GetUserWidgetObject (Variables|Default|GetWidget))))
  (Variables|Default|SetRotatingScoreWidget _asrotating_score)
  (CallFunction|SetNumbertoWidget (Variables|Default|GetScoreLeft))
  (Utilities|Time|SetTimerbyFunctionName 0 "UpdateScoringWidget" 0.1 true))

(fn ConstructionScript)

(fn SetNumbertoWidget
  (params (InNumber :type Integer))
  (Variables|/Game/Taeryong/Game/Widget/RotatingScore.RotatingScore_C|SetstrNameText (Variables|Default|GetRotatingScoreWidget) (Utilities|Text|ToText(Integer) InNumber)))

(fn UpdatingCountingLeft
  ;[1 1 1] 값이 바뀌면 적용된다
  (Variables|Default|SetScoreLeft (+ (Variables|Default|GetScoreLeft) 1)))

(fn UpdateScoringWidget
  (Transformation|SetWorldRotation (Variables|Default|GetWidget) (Math|Rotator|FindLookatRotation (Transformation|GetWorldLocation (Variables|Default|GetWidget)) (Camera|GetCameraLocation (Game|GetPlayerCameraManager 0))) false false)
  (Default|SetName (Variables|Default|GetRotatingScoreWidget) (Utilities|String|ToString(Integer) (Variables|Default|GetScoreLeft))))

(fn OnRepScoreLeft
  (CallFunction|SetNumbertoWidget (Variables|Default|GetScoreLeft))
  (Default|CallEventDispatcherUpdateCountLeft (Variables|Default|GetScoreLeft)))