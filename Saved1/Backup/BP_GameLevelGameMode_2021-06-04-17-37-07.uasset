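; Game mode Blueprint for the game level that numbers players as they join.
; When a new player starts, it increments a PlayerNum counter and writes the result to that player's BP_PlayerState.
; Korean debug prints show the count and the number assigned to the player.
; BeginPlay only calls the parent implementation.
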(event EventHandleStartingNewPlayer
  (params (NewPlayer :type Player%20Controller%20Object%20Reference))
  (bind _result (Math|Integer|IncrementInt (Variables|Default|GetPlayerNum))
    (:%20%20
      (Development|PrintString (Utilities|String|Append (Utilities|String|ToString(Integer) _result) "명"))
      (bind _asbp_player_state (Utilities|Casting|CastToBP_PlayerState (Variables|/Script/Engine.Controller|GetPlayerState NewPlayer)))
      (bind _output_get (Variables|/Game/Game/BP_PlayerState.BP_PlayerState_C|SetPlayerNum _asbp_player_state _result))
      (Development|PrintString (Utilities|String|Append (Utilities|GetDisplayName NewPlayer) "의 넘버는  " (Utilities|String|ToString(Integer) _output_get))))))

(event EventBeginPlay
  (|CallParentFunction))

(fn ConstructionScript)